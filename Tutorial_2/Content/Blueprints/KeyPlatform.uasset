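; Key platform actor in a maze game that lets the player collect its key with the Interact input.
; Overlapping the TriggerSound component enables input for the player's controller.
; Interact destroys the Key component, increments the player's key count and refreshes the HUD skulls through MazeGameMode.
; End overlap does nothing because the DisableInput logic is disconnected, so input stays enabled after leaving.
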(event OnComponentBeginOverlap(TriggerSound)
  (params (OverlappedComponent :type Primitive%20Component%20Object%20Reference) (OtherActor :type Actor%20Object%20Reference) (OtherComp :type Primitive%20Component%20Object%20Reference) (OtherBodyIndex :type Integer) (bFromSweep :type Boolean) (SweepResult :type Hit%20Result%20Structure%20%28by%20ref%29))
  (if (== OtherActor (Game|GetPlayerCharacter 0))
    (Input|EnableInput (Game|GetPlayerController 0))))

(event OnComponentEndOverlap(TriggerSound)
  (params (OverlappedComponent :type Primitive%20Component%20Object%20Reference) (OtherActor :type Actor%20Object%20Reference) (OtherComp :type Primitive%20Component%20Object%20Reference) (OtherBodyIndex :type Integer)))

(event Input|ActionEvents|InputActionInteract
  (params (Key :type Key%20Structure :default "None"))
  (:Pressed
    (Utilities|IsValid (Variables|Default|GetKey)
      (:Is%20Valid
        (Components|DestroyComponent (Variables|Default|GetKey))
        (bind _asplayer_character (Utilities|Casting|CastToPlayerCharacter (Game|GetPlayerCharacter 0)))
        (Math|Integer|IncrementInt (Variables|/Game/Player/PlayerCharacter.PlayerCharacter_C|GetNumberOfKeys _asplayer_character)
          (:%20%20
            (bind _asmaze_game_mode (Utilities|Casting|CastToMazeGameMode (Game|GetGameMode)))
            (Default|UpdateSkulls (Variables|/Game/GameSettings/MazeGameMode.MazeGameMode_C|GetHeadsUpDisplay _asmaze_game_mode))))))))

(fn ConstructionScript)