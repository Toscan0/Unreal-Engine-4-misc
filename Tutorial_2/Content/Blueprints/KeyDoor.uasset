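; A locked maze door that the player opens by spending a key.
; Overlapping its trigger while it is closed shows a HUD prompt and enables input if the player holds a key, otherwise a "Key missing" message.
; Interact decrements the key count, updates the HUD skulls, and snaps a newly added key mesh to the keyhole.
; A sound plays as a timeline moves key and door, then marks the door open.
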(event OnComponentEndOverlap(TriggerAudio)
  (params (OverlappedComponent :type Primitive%20Component%20Object%20Reference) (OtherActor :type Actor%20Object%20Reference) (OtherComp :type Primitive%20Component%20Object%20Reference) (OtherBodyIndex :type Integer))
  (if (== OtherActor (Game|GetPlayerCharacter 0))
    (Input|DisableInput (Game|GetPlayerController 0))
    (bind _asmaze_game_mode (Utilities|Casting|CastToMazeGameMode (Game|GetGameMode)))
    (Variables|/Game/UI/HeadsUpDisplay.HeadsUpDisplay_C|SetMessage (Variables|/Game/GameSettings/MazeGameMode.MazeGameMode_C|GetHeadsUpDisplay _asmaze_game_mode) "")
    (Default|UpdateMessage (Variables|/Game/GameSettings/MazeGameMode.MazeGameMode_C|GetHeadsUpDisplay _asmaze_game_mode))))

(event OnComponentBeginOverlap(TriggerAudio)
  (params (OverlappedComponent :type Primitive%20Component%20Object%20Reference) (OtherActor :type Actor%20Object%20Reference) (OtherComp :type Primitive%20Component%20Object%20Reference) (OtherBodyIndex :type Integer) (bFromSweep :type Boolean) (SweepResult :type Hit%20Result%20Structure%20%28by%20ref%29))
  (if (== OtherActor (Game|GetPlayerCharacter 0))
    (if (not (Variables|Default|GetIsOpen))
      (bind _asplayer_character (Utilities|Casting|CastToPlayerCharacter (Game|GetPlayerCharacter 0)))
      (if (> (Variables|/Game/Player/PlayerCharacter.PlayerCharacter_C|GetNumberOfKeys _asplayer_character) 0)
        (Input|EnableInput (Game|GetPlayerController 0))
        (bind _asmaze_game_mode (Utilities|Casting|CastToMazeGameMode (Game|GetGameMode)))
        (Variables|/Game/UI/HeadsUpDisplay.HeadsUpDisplay_C|SetMessage (Variables|/Game/GameSettings/MazeGameMode.MazeGameMode_C|GetHeadsUpDisplay _asmaze_game_mode) "Press 'E' to open door")
        (Default|UpdateMessage (Variables|/Game/GameSettings/MazeGameMode.MazeGameMode_C|GetHeadsUpDisplay _asmaze_game_mode))
        (else
          (bind _asmaze_game_mode_2 (Utilities|Casting|CastToMazeGameMode (Game|GetGameMode)))
          (Variables|/Game/UI/HeadsUpDisplay.HeadsUpDisplay_C|SetMessage (Variables|/Game/GameSettings/MazeGameMode.MazeGameMode_C|GetHeadsUpDisplay _asmaze_game_mode_2) "Key missing")
          (Default|UpdateMessage (Variables|/Game/GameSettings/MazeGameMode.MazeGameMode_C|GetHeadsUpDisplay _asmaze_game_mode_2)))))))

(event Input|ActionEvents|InputActionInteract
  (params (Key :type Key%20Structure :default "None"))
  (:Pressed
    (bind _asplayer_character (Utilities|Casting|CastToPlayerCharacter (Game|GetPlayerCharacter 0)))
    (if (> (Variables|/Game/Player/PlayerCharacter.PlayerCharacter_C|GetNumberOfKeys _asplayer_character) 0)
      (Math|Integer|DecrementInt (Variables|/Game/Player/PlayerCharacter.PlayerCharacter_C|GetNumberOfKeys _asplayer_character)
        (:%20%20
          (bind _asmaze_game_mode (Utilities|Casting|CastToMazeGameMode (Game|GetGameMode)))
          (Default|UpdateSkulls (Variables|/Game/GameSettings/MazeGameMode.MazeGameMode_C|GetHeadsUpDisplay _asmaze_game_mode))
          (bind _returnvalue (AddComponent|AddStaticMeshComponent false))
          (bind _output_get (Variables|Default|SetKeyMesh _returnvalue))
          (Transformation|AttachComponentToComponent _output_get (Variables|Default|GetKeyHole) "None" "SnapToTarget" "SnapToTarget" "SnapToTarget" true)
          (Audio|PlaySoundatLocation "/Game/Sounds/DoorOpening_SFX.DoorOpening_SFX" (Transformation|GetActorLocation) "0, 0, 0" 1.0 1.0 0.0 0 0 0)
          (bind (_direction _doorposition _keyposition) (Timeline|DoorOpening PlayFromStart)
            (:Update
              (Transformation|SetRelativeLocation (Variables|Default|GetKeyMesh) (Math|Vector|MakeVector 0.0 _keyposition 0.0) false false)
              (Transformation|SetRelativeLocation (Variables|Default|GetDoorMesh) (Math|Vector|MakeVector 0.0 0.0 _doorposition) false false)
              (bind _asmaze_game_mode_2 (Utilities|Casting|CastToMazeGameMode (Game|GetGameMode)))
              (Variables|/Game/UI/HeadsUpDisplay.HeadsUpDisplay_C|SetMessage (Variables|/Game/GameSettings/MazeGameMode.MazeGameMode_C|GetHeadsUpDisplay _asmaze_game_mode_2) "")
              (Default|UpdateMessage (Variables|/Game/GameSettings/MazeGameMode.MazeGameMode_C|GetHeadsUpDisplay _asmaze_game_mode_2)))
            (:Finished
              (Variables|Default|SetIsOpen true))))))))

(fn ConstructionScript)