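; An automatic door Blueprint that opens when the first player character enters its box trigger and closes when that character leaves.
; Two separate timelines, one per direction, each play from start and drive the door mesh's relative Z location.
; An IsOpen flag, set during timeline updates, gates each direction.
; The exit event also prints debug strings.
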(event OnComponentBeginOverlap(Box)
  (params (OverlappedComponent :type Primitive%20Component%20Object%20Reference) (OtherActor :type Actor%20Object%20Reference) (OtherComp :type Primitive%20Component%20Object%20Reference) (OtherBodyIndex :type Integer) (bFromSweep :type Boolean) (SweepResult :type Hit%20Result%20Structure%20%28by%20ref%29))
  (if (== OtherActor (Game|GetPlayerCharacter 0))
    (if (not (Variables|Default|GetisOpen))
      (bind _doorposition (Timeline|Timeline_0 PlayFromStart)
        (:Update
          (Transformation|SetRelativeLocation (Variables|Default|GetDoorMesh) (Math|Vector|MakeVector 0.0 0.0 _doorposition) false false)
          (Variables|Default|SetisOpen true))))))

(event OnComponentEndOverlap(Box)
  (params (OverlappedComponent :type Primitive%20Component%20Object%20Reference) (OtherActor :type Actor%20Object%20Reference) (OtherComp :type Primitive%20Component%20Object%20Reference) (OtherBodyIndex :type Integer))
  (if (== OtherActor (Game|GetPlayerCharacter 0))
    (Development|PrintString "Hello")
    (if (Variables|Default|GetisOpen)
      (Development|PrintString "2222")
      (bind _doorposition (Timeline|Timeline_1 PlayFromStart)
        (:Update
          (Transformation|SetRelativeLocation (Variables|Default|GetDoorMesh) (Math|Vector|MakeVector 0.0 0.0 _doorposition) false false)
          (Variables|Default|SetisOpen false))))))

(fn ConstructionScript)